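; BP_EnemySpawner repeatedly spawns BP_EnemyPawn enemies along the top edge of the player's orthographic camera view.
; On BeginPlay it reads the camera from BP_PlayerPawnSpace and computes horizontal Y limits and top Z from ortho width and viewport aspect ratio, once.
; An endless Delay loop then spawns an enemy at a random Y every SpawnDelay seconds, ignoring collisions.
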(event `Spawn Enemy`
  (`|SpawnActorFromClass` "/Game/BluePrints/BP_EnemyPawn.BP_EnemyPawn_C" (`KismetMathLibrary.MakeTransform` (`KismetMathLibrary.MakeVector` 0.0 (`KismetMathLibrary.RandomFloatInRange` (`self.YMin`) (`self.YMax`)) (`self.Z Spawn`))) "AlwaysSpawn" "MultiplyWithRoot" null null))

(event `self.ReceiveBeginPlay`
  (bind _asbp_player_pawn_space (cast `/Game/BluePrints/BP_PlayerPawnSpace` (`GameplayStatics.GetPlayerPawn` 0)))
  (`self.Set Viewport Limits` (`/Game/BluePrints/BP_PlayerPawnSpace.PlayerCamera Reference` _asbp_player_pawn_space))
  (`self.Spawn Enemy` :!label _label)
  (`KismetSystemLibrary.Delay` (`self.Spawn Delay`))
  (goto _label))

(event `Set Viewport Limits`
  (params (Camera :type "CameraComponent Object Reference"))
  (bind _returnvalue (`SceneComponent.K2_GetComponentLocation` Camera))
  (bind (_returnvalue_x _returnvalue_y) (`KismetMathLibrary.BreakVector2D` (`WidgetLayoutLibrary.GetViewportSize`)))
  (bind _orthowidth (`CameraComponent.OrthoWidth` Camera))
  (bind (_returnvalue_x_2 _returnvalue_y_2) (`KismetMathLibrary.BreakVector` (- _returnvalue (* (* _orthowidth 0.5) (0.0 1.0 0.0)))))
  (bind (_returnvalue_x_3 _returnvalue_y_3 _returnvalue_z) (`KismetMathLibrary.BreakVector` (+ _returnvalue (* (* (/ _orthowidth (/ _returnvalue_x _returnvalue_y)) 0.5) (0.0 0.0 1.0)))))
  (bind _output_get (set `self.YMin` _returnvalue_y_2))
  (set `self.YMax` (+ _output_get _orthowidth))
  (set `self.Z Spawn` _returnvalue_z))

(fn `UserConstructionScript`)