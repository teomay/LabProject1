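; BP_GameStateSpace is a game state Blueprint that tracks the score and game-over flag and drives the main UI.
; On BeginPlay it creates WBP_MainUI for the first player controller, stores it and adds it to the viewport.
; IncreaseScore adds points and pushes the new total to the widget, while GameOver sets the flag and tells the widget to show its game-over UI.
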(event `self.ReceiveBeginPlay`
  (bind _returnvalue (`|CreateWidget` "/Game/BluePrints/WBP_MainUI.WBP_MainUI_C" (`GameplayStatics.GetPlayerController` 0)))
  (bind _output_get (set `self.MainUI` _returnvalue))
  (`UserWidget.AddToViewport` _output_get 0))

(event `Increase Score`
  (params (`Point Value` :type Integer))
  (bind _output_get (set `self.Score` (+ `Point Value` (`self.Score`))))
  (`/Game/BluePrints/WBP_MainUI.Update Score Text` (`self.MainUI`) _output_get))

(event `GameOver`
  (set `self.Is Game Over?` true)
  (`/Game/BluePrints/WBP_MainUI.Show Game Over UI` (`self.MainUI`)))

(fn `UserConstructionScript`)